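; BP_Cap02 is an interactive actor whose Box trigger opens the WG_Cap02 widget and drives animation on the SkCap02 component.
; On overlap it adds the widget to the viewport, shows the mouse cursor, disables player pawn input and hands the widget a self-reference.
; EV_Ani sets and plays a non-looping animation, with no caller in this Blueprint.
; End overlap zeroes the play rate and calls a non-looping Play.
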(event OnComponentBeginOverlap(Box)
  (params (OverlappedComponent :type Primitive%20Component%20Object%20Reference) (OtherActor :type Actor%20Object%20Reference) (OtherComp :type Primitive%20Component%20Object%20Reference) (OtherBodyIndex :type Integer) (bFromSweep :type Boolean) (SweepResult :type Hit%20Result%20Structure%20%28by%20ref%29))
  (bind _returnvalue (Game|GetPlayerController 0))
  (bind _returnvalue_2 (UserInterface|CreateWidget "/Game/SM03/WG_Cap02.WG_Cap02_C" (Game|GetPlayerController 0)))
  (UserInterface|Viewport|AddtoViewport _returnvalue_2 0)
  (Variables|/Script/Engine.PlayerController|SetbShowMouseCursor _returnvalue true)
  (Input|DisableInput (Game|Player|GetPlayerPawn 0) _returnvalue)
  (Variables|/Game/SM03/WG_Cap02.WG_Cap02_C|Set응애 _returnvalue_2 self))

(event OnComponentEndOverlap(Box)
  (params (OverlappedComponent :type Primitive%20Component%20Object%20Reference) (OtherActor :type Actor%20Object%20Reference) (OtherComp :type Primitive%20Component%20Object%20Reference) (OtherBodyIndex :type Integer))
  (Components|Timeline|SetPlayRate (Variables|Default|GetSk_cap02) 0.0)
  (Audio|Components|Audio|Play (Variables|Default|GetSk_cap02) false))

(event Custom|EV_Ani
  (Components|Animation|SetAnimation (Variables|Default|GetSk_cap02) 0)
  (Components|Animation|PlayAnimation (Variables|Default|GetSk_cap02) 0 false))

(fn ConstructionScript)