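; BP_Box2 is an interactable actor that opens a WG_Open widget when its Box trigger is overlapped and can swing its Cube open.
; The overlap shows the mouse cursor, disables input on the player pawn and passes the actor to the widget as DD.
; EV_Act, not called within this Blueprint, plays a timeline that lerps the Cube's relative yaw from 0 to 120 degrees.
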(event OnComponentBeginOverlap(Box)
  (params (OverlappedComponent :type Primitive%20Component%20Object%20Reference) (OtherActor :type Actor%20Object%20Reference) (OtherComp :type Primitive%20Component%20Object%20Reference) (OtherBodyIndex :type Integer) (bFromSweep :type Boolean) (SweepResult :type Hit%20Result%20Structure%20%28by%20ref%29))
  (bind _returnvalue (Game|GetPlayerController 0))
  (bind _returnvalue_2 (UserInterface|CreateWidget "/Game/SM03/WG_Open.WG_Open_C" (Game|GetPlayerController 0)))
  (UserInterface|Viewport|AddtoViewport _returnvalue_2 0)
  (Variables|/Script/Engine.PlayerController|SetbShowMouseCursor _returnvalue true)
  (Input|DisableInput (Game|Player|GetPlayerPawn 0) _returnvalue)
  (Variables|/Game/SM03/WG_Open.WG_Open_C|SetDD _returnvalue_2 self))

(event Custom|EV_Act
  (bind _newtrack_0 (Timeline|Timeline PlayFromStart)
    (:Update
      (Transformation|SetRelativeRotation (Variables|Default|GetCube) (Math|Rotator|MakeRotator 0.0 0.0 (Math|Float|Lerp 0.0 1.2e+02 _newtrack_0)) false false))))

(fn ConstructionScript)